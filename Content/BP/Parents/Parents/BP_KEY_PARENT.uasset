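; Base Blueprint for a collectible key pickup that comes in red, green or blue.
; The construction script sets the key mesh's metal material from KeyType.
; BeginPlay binds to the ItemPickedUp dispatcher, whose handler plays the key drop sound, reports one key of that type to the GameInstance, then destroys the actor.
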(event `self.ReceiveBeginPlay`
  (`parent.ReceiveBeginPlay`)
  (add `self.ItemPickedUp` (delegate `ItemPickedUp_Event`)))

(event `ItemPickedUp_Event`
  (`GameplayStatics.PlaySoundAtLocation` "/Game/Sounds/KeyDrop.KeyDrop" (`self.K2_GetActorLocation`) (struct) 1.0 1.0 0.5 null null null null)
  (message `/Game/BP/Interfaces/BPI_PlayerInfo.UpdateKeysAmount` (`GameplayStatics.GetGameInstance`) (`self.KeyType`) 1)
  (`self.K2_DestroyActor`))

(fn `UserConstructionScript`
  (`parent.UserConstructionScript`)
  (`PrimitiveComponent.SetMaterial` (`self.Key`) 0 (select `/Game/BP/MISC/E_Keytypes` (`self.KeyType`) :`NewEnumerator0` "/Game/Materials/MI_Metal_Red.MI_Metal_Red" :`NewEnumerator1` "/Game/Materials/MI_Metal_Green.MI_Metal_Green" :`NewEnumerator2` "/Game/Materials/MI_Metal_Blue.MI_Metal_Blue" :!type "MaterialInterface Object Reference")))