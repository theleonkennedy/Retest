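; Parent pickup actor that broadcasts ItemPickedUp when the player character overlaps its collision with touch pickup enabled, or when Interact fires.
; BeginPlay toggles bobbing (InterpToMovement) and spinning (RotatingMovement), optionally randomizing both within set ranges.
; The construction script configures the point light and places it near the collision sphere's bottom.
; GetInteractionInfo exposes interaction data; the custom depth stencil setter is disconnected.
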(event `self.ReceiveBeginPlay`
  (bind _interptomovement (`self.InterpToMovement`))
  (`|ExecutionSequence`
    (:`then_0`
      ; Activate/Deactivate Movements
      (`ActorComponent.SetActive` (`self.InterpToMovement`) (`self.Active Bob`) false)
      (`ActorComponent.SetActive` (`self.RotatingMovement`) (`self.Active Rotate`) false)
      ; Set all static mesh components to vvalue of 1 for custom depth stencil value
      (for _array_element (`|MakeArray` (`self.GetComponentByClass` "/Script/Engine.StaticMeshComponent"))
        _))
    (:`then_1`
      ; Randomize movements
      (if (`self.Randomize Movement`)
        ;; Randomize bob amount and duration
        (set `InterpToMovementComponent.Duration` (`KismetMathLibrary.RandomFloatInRange` (`self.MinBobDuration`) (`self.MaxBobDuration`)) _interptomovement)
        (`KismetArrayLibrary.Array_Set` (`InterpToMovementComponent.ControlPoints` _interptomovement) 0 (make `InterpControlPoint` (`KismetMathLibrary.MakeVector` 0.0 0.0 (`KismetMathLibrary.RandomFloatInRange` (`self.MinBobAmount`) (`self.MaxBobAmount`)))) true)
        ;; Randomize rotation amount
        (set `RotatingMovementComponent.RotationRate` (`KismetMathLibrary.MakeRotator` 0.0 0.0 (`KismetMathLibrary.RandomFloatInRange` (`self.MinRotationAmount`) (`self.MaxRotateAmouunt`))) (`self.RotatingMovement`))))))

(event `self.Collision.OnComponentBeginOverlap`
  (params (OverlappedComponent :type "PrimitiveComponent Object Reference") (OtherActor :type "Actor Object Reference") (OtherComp :type "PrimitiveComponent Object Reference") (OtherBodyIndex :type Integer) (bFromSweep :type Boolean) (SweepResult :type "HitResult Structure (by ref)"))
  ; Trigger picked by player
  (if (and (== OtherActor (`GameplayStatics.GetPlayerCharacter` 0)) (`self.TouchPickUpActive`))
    (`self.ItemPickedUp` :!label _label)))

(event `/Game/BP/Interfaces/BPI_Interaction.Interact`
  ; Trigger picked by player
  (goto _label))

(fn `GetInteractionInfo`
  (returns (InteractionInfo :type Text))
  (return (`self.Interaction Info`)))

(fn `UserConstructionScript`
  (bind _pointlight (`self.PointLight`))
  (`SceneComponent.K2_SetRelativeLocation` _pointlight (`KismetMathLibrary.MakeVector` 0.0 0.0 (* (`SphereComponent.SphereRadius` (`self.Collision`)) -0.9)) false false)
  (`LightComponent.SetLightColor` _pointlight (`self.New Light Color`) true)
  (`LightComponent.SetIntensity` _pointlight (`self.Light Intensity`))
  (`SceneComponent.SetVisibility` _pointlight (`self.LightActive`) false))