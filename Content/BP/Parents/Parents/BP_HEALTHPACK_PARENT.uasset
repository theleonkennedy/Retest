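; Parent Blueprint for health pack pickups that heal the player when picked up.
; It binds to ItemPickedUp, checks the player's AC_Health, and heals by applying negative HealAmount as damage, then plays a sound chosen by the returned damage's sign and destroys itself.
; At full health it stays and shows a HUD notification instead.
; The construction script applies configurable materials to the base and cross meshes.
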(event `self.ReceiveBeginPlay`
  (`parent.ReceiveBeginPlay`)
  (add `self.ItemPickedUp` (delegate `ItemPickedUp_Event`)))

(event `ItemPickedUp_Event`
  (bind _returnvalue (`GameplayStatics.GetPlayerCharacter` 0))
  (bind _returnvalue_2 (`self.GetComponentByClass` _returnvalue "/Game/BP/Component/AC_Health.AC_Health_C"))
  (`/Engine/EditorBlueprintResources/StandardMacros.IsValid` _returnvalue_2
    (:`Is Valid`
      (if (< (`/Game/BP/Component/AC_Health.Health` _returnvalue_2) (`/Game/BP/Component/AC_Health.MaxHealth` _returnvalue_2))
        (bind _returnvalue_3 (`GameplayStatics.ApplyDamage` _returnvalue (* (`self.HealAmount`) -1.0)))
        (`GameplayStatics.PlaySoundAtLocation` (select `bool` (>= _returnvalue_3 0.0) :`false` "/Game/Sounds/yes-2_Cue.yes-2_Cue" :`true` "/Game/Sounds/MaleCough_Cue.MaleCough_Cue" :!type "SoundBase Object Reference") (`self.K2_GetActorLocation` _returnvalue) (struct) 1.0 1.0 0.0 null null null null)
        (`self.K2_DestroyActor`)
        (else
          (message `/Game/BP/Interfaces/BPI_Interaction.UpdateHUD_Notification` (`GameplayStatics.GetPlayerController` 0) "HealthFull"))))))

(fn `UserConstructionScript`
  (`parent.UserConstructionScript`)
  (`PrimitiveComponent.SetMaterial` (`self.BasePack`) 0 (`self.BaseMaterial`))
  (`PrimitiveComponent.SetMaterial` (`self.Cross02`) 0 (`self.CrossMaterial`))
  (`PrimitiveComponent.SetMaterial` (`self.Cross03`) 0 (`self.CrossMaterial`))
  (`PrimitiveComponent.SetMaterial` (`self.Cross04`) 0 (`self.CrossMaterial`))
  (`PrimitiveComponent.SetMaterial` (`self.Cross01`) 0 (`self.CrossMaterial`)))