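; BP_HEALTHPACK_PARENT is a pickup Blueprint that, despite its health pack name, behaves as a coin.
; On BeginPlay it binds to the inherited ItemPickedUp dispatcher, whose event prints the pickup Value, plays a coin sound at its location and destroys the actor.
; The Construction Script runs the parent's version, then applies the coin material to the BasePack component.
; No healing logic appears in these graphs.
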(event `self.ReceiveBeginPlay`
  (`parent.ReceiveBeginPlay`)
  (add `self.ItemPickedUp` (delegate `ItemPickedUp_Event`)))

(event `ItemPickedUp_Event`
  (`KismetSystemLibrary.PrintText` (`|FormatText` "Coin picked up for value {x}" (`self.Value`)))
  (`GameplayStatics.PlaySoundAtLocation` "/Game/Sounds/coin_2.coin_2" (`self.K2_GetActorLocation`) (struct) 1.0 1.0 0.0 null null null null)
  (`self.K2_DestroyActor`))

(fn `UserConstructionScript`
  (`parent.UserConstructionScript`)
  (`PrimitiveComponent.SetMaterial` (`self.BasePack`) 0 (`self.CoinMaterial`)))