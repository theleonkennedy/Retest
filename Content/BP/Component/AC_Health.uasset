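; Actor component that tracks its owner's health, binding to the owner's any-damage event on BeginPlay.
; Damage is subtracted from Health with only an upper clamp at MaxHealth, so negative damage heals.
; The result fires dispatchers for health received, damage taken or health at or below zero.
; Owners without a player-controlled Instigator get an initially hidden screen-space WBP_Healthbar, created a tick later above their bounds.
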(event `self.ReceiveBeginPlay`
  (bind _returnvalue (`self.GetOwner`))
  ; Auto-assign TkaeAnyDamage to owner
  (add `Actor.OnTakeAnyDamage` (`self.GetOwner`) (delegate `OnTakeAnyDamage_Event`))
  ; Check if owned actor is player controlled
  (`KismetSystemLibrary.DelayUntilNextTick`)
  (bind _instigator (`Actor.Instigator` (`self.GetOwner`))
    (:`then`
      (if (not (`Pawn.IsPlayerControlled` _instigator))
        ; Create healthbar widget above object // Only visible when taking damage
        (bind _returnvalue_2 (`|AddComponentByClass` _returnvalue "/Script/UMG.WidgetComponent" false (`KismetMathLibrary.MakeTransform` (`KismetMathLibrary.MakeVector` 0.0 0.0 (+ (.z (`.BoxExtent` (`Actor.GetActorBounds` _returnvalue false false))) (`self.HealthbarHeightOffset`)))) :!label _label))
        (bind _output_get (set `self.WidgetComp` _returnvalue_2))
        (`WidgetComponent.SetDrawSize` _output_get (100.0 10.0))
        (`WidgetComponent.SetWidgetSpace` _output_get "Screen")
        (`PrimitiveComponent.SetCollisionEnabled` _output_get "NoCollision")
        (`SceneComponent.SetHiddenInGame` _output_get true false)
        (bind _returnvalue_3 (`|CreateWidget` "/Game/UI/WBP_Healthbar.WBP_Healthbar_C"))
        (bind _output_get_2 (set `self.WBP Healthbar` _returnvalue_3))
        (`WidgetComponent.SetWidget` _output_get _output_get_2)))
    (:`else`
      (goto _label))))

(event `OnTakeAnyDamage_Event`
  (params (DamagedActor :type "Actor Object Reference") (Damage :type "Float (single-precision)") (DamageType :type "DamageType Object Reference") (InstigatedBy :type "Controller Object Reference") (DamageCauser :type "Actor Object Reference"))
  ; Auto-assign TkaeAnyDamage to owner
  (`self.ProcessDamage` Damage))

(event `ProcessDamage`
  (params (Damage :type "Float (double-precision)"))
  ; Process incoming damage
  (bind (_results _healing) (`self.DamageIntake` Damage))
  (if _healing
    (`self.OnHealthRecieve`)
    (else
      (`/Engine/EditorBlueprintResources/StandardMacros.CompareFloat` _results
        (:`>`
          (`self.OnDamageTaken`))
        (:`==`
          (`self.OnHealthZero` :!label _label_2))
        (:`<`
          (goto _label_2))))))

(fn `DamageIntake`
  (params (Damage :type "Float (double-precision)"))
  (returns (Results :type "Float (double-precision)") (Healing :type Boolean))
  (bind _output_get (set `self.Health` (`KismetMathLibrary.FMin` (- (`self.Health`) Damage) (`self.MaxHealth`))))
  (return _output_get (< (`local.Damage`) 0.0)))