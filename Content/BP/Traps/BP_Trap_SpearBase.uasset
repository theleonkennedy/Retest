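; Spear trap base that, when its linked trigger activates, fires spear projectiles upward in a random cone if deployed, then reverses the deploy timeline.
; The construction script builds an instanced spear grid and fits the damage box and optional platform to it.
; Overlapping the box damages characters and launches them up and back.
; Timeline update and redeploy logic is unwired, and the collision toggle always selects NoCollision.
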(event `self.ReceiveBeginPlay`
  ; Fire spears from trigger
  (bind _traptrigger (`self.TrapTrigger`)
    (:`then`
      (add `/Game/BP/Traps/BP_TrapTrigger.OnActivateTrap` _traptrigger (delegate `OnActivateTrap_Event`)))
    (:`else`)))

(event `OnActivateTrap_Event`
  (bind _spears (`self.Spears`))
  ; Fire spears from trigger
  (if (`self.Spearseployed`)
    (for _index (range (`InstancedStaticMeshComponent.GetInstanceCount` _spears))
      (`|SpawnActorFromClass` "/Game/BP/Traps/BP_Proj_Spears.BP_Proj_Spears_C" (`KismetMathLibrary.MakeTransform` (.location (`InstancedStaticMeshComponent.GetInstanceTransform` _spears _index true)) (`KismetMathLibrary.Conv_VectorToRotator` (`KismetMathLibrary.RandomUnitVectorInConeInDegrees` (`self.GetActorUpVector`) (`self.SpearAngleShotVariation`)))) "AlwaysSpawn" "MultiplyWithRoot" null (`self.SpearLaunchSpeed`) null)
      (`AudioComponent.Play` (`self.Audio_SpearFire`) 0.0))
    (`self.SpearDeploymentSpeed` (`self.SpearRetractsSpeed`))
    (`TimelineComponent.ReverseFromEnd` (`self.TL_DeploySpears`))))

(event `self.PainCollision.OnComponentBeginOverlap`
  (params (OverlappedComponent :type "PrimitiveComponent Object Reference") (OtherActor :type "Actor Object Reference") (OtherComp :type "PrimitiveComponent Object Reference") (OtherBodyIndex :type Integer) (bFromSweep :type Boolean) (SweepResult :type "HitResult Structure (by ref)"))
  ; Apply damage to character hit by spikes
  (bind _ascharacter (cast `Character` OtherActor))
  (`GameplayStatics.ApplyDamage` _ascharacter (`self.DamageAmount`))
  ; Push back character after taking damage
  (`Character.LaunchCharacter` _ascharacter (* (/ (+ (`self.GetActorUpVector` _ascharacter) (* (`self.GetActorForwardVector` _ascharacter) -1)) 2) (`self.DamageLaunchStrenght`)) true true))

(fn `CreateSpears`
  (locals (SpikeTransforms :type "Array of Transform Structure"))
  (bind _spacing (`self.Spacing`))
  (bind _spacing_2 (`self.Spacing`))
  (bind _spears (`self.Spears`))
  ; Create Spike Grid
  (for _index (range 1 (+ (`self.SpikeGridSizeY`) 1))
    (for _index_2 (range 1 (+ (`self.SpikeGridSizeX`) 1))
      (`KismetArrayLibrary.Array_Add` (`local.SpikeTransforms`) (`KismetMathLibrary.MakeTransform` (`KismetMathLibrary.MakeVector` (+ (* _index_2 _spacing -1.0) _spacing) (+ (* _index _spacing_2 -1.0) _spacing_2)) (struct) (0.1 0.1 1.0)))))
  (`InstancedStaticMeshComponent.AddInstances` _spears (`local.SpikeTransforms`) false false true)
  (`SceneComponent.K2_SetRelativeLocation` _spears (`KismetMathLibrary.MakeVector` (* (- (`self.SpikeGridSizeX`) 1) (`self.Spacing`) 0.5) (* (- (`self.SpikeGridSizeY`) 1) (`self.Spacing`) 0.5)) false false))

(fn `EnablePainColision`
  (params (Index :type Boolean))
  (`PrimitiveComponent.SetCollisionEnabled` (`self.PainCollision`) (select `bool` Index :`false` "NoCollision" :`true` "NoCollision" :!type "ECollisionEnabled Enum")))

(fn `PlayRetractionAudio`
  (params (VolumeMultiplier :type "Float (single-precision)" :default 1.0) (PitchMultiplier :type "Float (single-precision)" :default 1.0))
  (bind _audio_spearsretract (`self.Audio_SpearsRetract`))
  (`AudioComponent.SetVolumeMultiplier` _audio_spearsretract VolumeMultiplier)
  (`AudioComponent.SetPitchMultiplier` _audio_spearsretract PitchMultiplier)
  (`AudioComponent.Play` _audio_spearsretract 0.0))

(fn `SetTrapPositionForClipping`
  (bind _spears (`self.Spears`))
  (`MeshComponent.SetVectorParameterValueOnMaterials` _spears "ClipPosition" (`self.K2_GetActorLocation`))
  (`MeshComponent.SetVectorParameterValueOnMaterials` _spears "ClipUpVector" (`self.GetActorUpVector`)))

(fn `SpearDeploymentSpeed`
  (params (DeploymentSpeed :type "Float (double-precision)" :default 0.1))
  (`TimelineComponent.SetPlayRate` (`self.TL_DeploySpears`) (/ 1.0 DeploymentSpeed)))

(fn `UserConstructionScript`
  (bind _paincollision (`self.PainCollision`))
  (bind _platform (`self.Platform`))
  (bind _spears (`self.Spears`))
  (bind (_min _max) (`StaticMeshComponent.GetLocalBounds` _spears))
  (bind _returnvalue (+ (* (/ (- _max _min) 2) (.scale (`InstancedStaticMeshComponent.GetInstanceTransform` _spears 0 false))) (`KismetMathLibrary.MakeVector` (* (- (`self.SpikeGridSizeX`) 1) (`self.Spacing`) 0.5) (* (- (`self.SpikeGridSizeY`) 1) (`self.Spacing`) 0.5))))
  (bind (_returnvalue_x _returnvalue_y) (`KismetMathLibrary.BreakVector` (/ (+ _returnvalue (`self.PlatformSizeBuffer`)) 50)))
  ; Create dynamic spikes layout and adjust PainCollision to automatically fit the bounds of the spikes
  (`self.CreateSpears`)
  (`BoxComponent.SetBoxExtent` _paincollision _returnvalue true)
  (`SceneComponent.K2_SetRelativeLocation` _paincollision (`KismetMathLibrary.MakeVector` 0.0 0.0 (.z _returnvalue)) false false)
  ; Set size and visibility of platform
  (`SceneComponent.SetRelativeScale3D` _platform (`KismetMathLibrary.MakeVector` _returnvalue_x _returnvalue_y 0.05))
  (`SceneComponent.SetHiddenInGame` _platform (`self.HidePlatform`) false))