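; BP_TrapTrigger is a trigger volume with a platform that activates traps when the player steps into it.
; On overlap by player character 0, it calls the OnActivateTrap dispatcher for connected traps to respond.
; The construction script sizes and raises the box from CollisionExtents, scales a thin platform to match, optionally hides it in game, and resets the text label's world rotation.
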(event `self.Collision.OnComponentBeginOverlap`
  (params (OverlappedComponent :type "PrimitiveComponent Object Reference") (OtherActor :type "Actor Object Reference") (OtherComp :type "PrimitiveComponent Object Reference") (OtherBodyIndex :type Integer) (bFromSweep :type Boolean) (SweepResult :type "HitResult Structure (by ref)"))
  ; Trigger connect traps when trigger is activated
  (if (== OtherActor (`GameplayStatics.GetPlayerCharacter` 0))
    (`self.OnActivateTrap`)))

(fn `UserConstructionScript`
  (bind _collisionextents (`self.CollisionExtents`))
  (bind _platform (`self.Platform`))
  (bind _collision (`self.Collision`))
  (bind (_returnvalue_x _returnvalue_y) (`KismetMathLibrary.BreakVector` (/ _collisionextents 50)))
  ; Set Size and location of collision
  (`BoxComponent.SetBoxExtent` _collision _collisionextents true)
  (`SceneComponent.K2_SetRelativeLocation` _collision (`KismetMathLibrary.MakeVector` 0.0 0.0 (.z _collisionextents)) false false)
  ; Set size and visibility of platform
  (`SceneComponent.SetRelativeScale3D` _platform (`KismetMathLibrary.MakeVector` _returnvalue_x _returnvalue_y 0.05))
  (`SceneComponent.SetHiddenInGame` _platform (`self.HidePlatform`) false)
  (`SceneComponent.K2_SetWorldRotation` :`self` (`self.TextRender`)) ; Prevents text from spinning
)