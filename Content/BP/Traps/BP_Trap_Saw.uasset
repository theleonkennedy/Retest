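; Saw blade trap that slides along a configurable railing, damaging and launching back characters it overlaps.
; The construction script sizes rail and blade, derives padded travel extents and places the blade at its starting point.
; Travel uses a timeline with fixed or randomized duration, started on BeginPlay if active or by an optional TrapTrigger.
; Activation also enables overlap collision and spins the blade through a material parameter.
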(event `self.ReceiveBeginPlay`
  (`|ExecutionSequence`
    (:`then_0`
      ; Set new time for saw movement to starting point of the blad
      (`TimelineComponent.SetNewTime` (`self.TL_SawMovement`) (`self.BladeStartingPoint`)))
    (:`then_1`
      ; Set for blade to travel across railing one way
      (`TimelineComponent.SetPlayRate` (`self.TL_SawMovement`) (/ 1.0 (select `bool` (`self.RandomizedBladeTravelTime`) :`false` (`self.SawBladeTravelTime`) :`true` (`KismetMathLibrary.RandomFloatInRange` (`self.MinSawBladeTravelTime`) (`self.MaxSawBladeTravelTime`))))))
    (:`then_2`
      ; Activate saw blade with trap trigger
      (bind _traptrigger (`self.TrapTrigger`)
        (:`then`
          (add `/Game/BP/Traps/BP_TrapTrigger.OnActivateTrap` _traptrigger (delegate `OnActivateTrap_Event`)))
        (:`else`)))
    (:`then_3`
      ; Auto activate saw movement
      (if (`self.IsActive`)
        (`self.ActivateSaw`)
        (else
          (`MeshComponent.SetScalarParameterValueOnMaterials` (`self.SawBlade`) "RotationSpeed" 0.0))))))

(event `OnActivateTrap_Event`
  ; Activate saw blade with trap trigger
  (set `self.IsActive` true)
  (`self.ActivateSaw`))

(event `self.SawBlade.OnComponentBeginOverlap`
  (params (OverlappedComponent :type "PrimitiveComponent Object Reference") (OtherActor :type "Actor Object Reference") (OtherComp :type "PrimitiveComponent Object Reference") (OtherBodyIndex :type Integer) (bFromSweep :type Boolean) (SweepResult :type "HitResult Structure (by ref)"))
  ; Apply damage to character hit by blade
  (bind _ascharacter (cast `Character` OtherActor))
  (`GameplayStatics.ApplyDamage` _ascharacter (`self.DamageAmount`))
  ; Push back character after taking damage
  (`Character.LaunchCharacter` _ascharacter (* (/ (+ (`self.GetActorUpVector` _ascharacter) (* (`self.GetActorForwardVector` _ascharacter) -1)) 2) (`self.DamageLaunchStrenght`)) true true))

(event `ActivateSaw`
  ; Activate saw movement and damage ability
  (`PrimitiveComponent.SetCollisionResponseToAllChannels` (`self.SawBlade`) "ECR_Overlap")
  (`TimelineComponent.Play` (`self.TL_SawMovement`))
  (`MeshComponent.SetScalarParameterValueOnMaterials` (`self.SawBlade`) "RotationSpeed" -1.0))

(fn `CalculateSawBladeMovementExtents`
  (set `self.SawBladeMovementExtent` (- (/ (`self.RailLength`) 2.0) (`.SphereRadius` (`KismetSystemLibrary.GetComponentBounds` (`self.SawBlade`))) (`self.RailLenghtBladePadding`))))

(fn `UserConstructionScript`
  (bind _sawbladescale (`self.SawBladeScale`))
  (bind _sawblade (`self.SawBlade`))
  (bind _sawblademovementextent (`self.SawBladeMovementExtent`))
  (`SceneComponent.SetRelativeScale3D` (`self.Railing`) (`KismetMathLibrary.MakeVector` (/ (`self.RailLength`) 100.0) 0.1 0.1))
  (`SceneComponent.SetRelativeScale3D` _sawblade (`KismetMathLibrary.MakeVector` _sawbladescale 1.0 _sawbladescale))
  (`self.CalculateSawBladeMovementExtents`)
  (`SceneComponent.K2_SetRelativeLocation` _sawblade (`KismetMathLibrary.MakeVector` (`KismetMathLibrary.Lerp` _sawblademovementextent (* _sawblademovementextent -1.0) (`self.BladeStartingPoint`))) false false))