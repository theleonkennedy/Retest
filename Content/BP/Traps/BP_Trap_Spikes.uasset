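; Spike trap that deploys when a character overlaps it while armed, damaging and launching characters that hit its pain box.
; An optional TrapTrigger arms it, otherwise it arms on BeginPlay.
; A timeline drives deployment and optional delayed retraction, with audio.
; The construction script builds an instanced spike grid, fits platform and collision boxes to its bounds, and feeds actor position and up vector to materials for clipping.
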(event `OnActivateTrap_Event`
  ; Arm trap from trigger
  (set `self.IsArmed` true :!label _label))

(event `self.ReceiveBeginPlay`
  (`|ExecutionSequence`
    (:`then_0`
      ; Arm trap from trigger
      (bind _traptrigger (`self.TrapTrigger`)
        (:`then`
          (add `/Game/BP/Traps/BP_TrapTrigger.OnActivateTrap` _traptrigger (delegate `OnActivateTrap_Event`)))
        (:`else`
          (goto _label))))
    (:`then_1`
      (`self.SpikeDeploymentSpeed` 0.1) ; How fast the spikes deploy
    )))

(event `self.TriggerCollision.OnComponentBeginOverlap`
  (params (OverlappedComponent :type "PrimitiveComponent Object Reference") (OtherActor :type "Actor Object Reference") (OtherComp :type "PrimitiveComponent Object Reference") (OtherBodyIndex :type Integer) (bFromSweep :type Boolean) (SweepResult :type "HitResult Structure (by ref)"))
  ; Deploy spikes when triggered by character
  (cast `Character` OtherActor)
  (if (and (`self.IsArmed`) (not (`self.SpikesDeployed`)))
    (`TimelineComponent.Play` (`self.TL_DeploySpikes`))
    (`self.PlayAudio` 1.0)))

(event `self.PainCollision.OnComponentBeginOverlap`
  (params (OverlappedComponent :type "PrimitiveComponent Object Reference") (OtherActor :type "Actor Object Reference") (OtherComp :type "PrimitiveComponent Object Reference") (OtherBodyIndex :type Integer) (bFromSweep :type Boolean) (SweepResult :type "HitResult Structure (by ref)"))
  ; Apply damage to character hit by spikes
  (bind _ascharacter (cast `Character` OtherActor))
  (`GameplayStatics.ApplyDamage` _ascharacter (`self.DamageAmount`))
  ; Push back character after taking damage
  (`Character.LaunchCharacter` _ascharacter (* (/ (+ (`self.GetActorUpVector` _ascharacter) (* (`self.GetActorForwardVector` _ascharacter) -1)) 2) (`self.DamageLaunchStrenght`)) true true))

(fn `CreateSpikes`
  (locals (SpikeTransforms :type "Array of Transform Structure"))
  (bind _spacing (`self.Spacing`))
  (bind _spacing_2 (`self.Spacing`))
  (bind _spikes (`self.Spikes`))
  ; Create Spike Grid
  (for _index (range 1 (+ (`self.SpikeGridSizeY`) 1))
    (for _index_2 (range 1 (+ (`self.SpikeGridSizeX`) 1))
      (`KismetArrayLibrary.Array_Add` (`local.SpikeTransforms`) (`KismetMathLibrary.MakeTransform` (`KismetMathLibrary.MakeVector` (+ (* _index_2 _spacing -1.0) _spacing) (+ (* _index _spacing_2 -1.0) _spacing_2)) (struct) (0.1 0.1 1.0)))))
  (`InstancedStaticMeshComponent.AddInstances` _spikes (`local.SpikeTransforms`) false false true)
  (`SceneComponent.K2_SetRelativeLocation` _spikes (`KismetMathLibrary.MakeVector` (* (- (`self.SpikeGridSizeX`) 1) (`self.Spacing`) 0.5) (* (- (`self.SpikeGridSizeY`) 1) (`self.Spacing`) 0.5)) false false))

(fn `EnablePainCollision`
  (params (Index :type Boolean))
  (`PrimitiveComponent.SetCollisionEnabled` (`self.PainCollision`) (select `bool` Index :`false` "NoCollision" :`true` "NoCollision" :!type "ECollisionEnabled Enum")))

(fn `PlayAudio`
  (params (VolumeMultiplier :type "Float (single-precision)" :default 1.0) (PitchMultiplier :type "Float (single-precision)" :default 1.0))
  (bind _audio_spikes (`self.Audio_Spikes`))
  (`AudioComponent.SetVolumeMultiplier` _audio_spikes VolumeMultiplier)
  (`AudioComponent.SetPitchMultiplier` _audio_spikes PitchMultiplier)
  (`AudioComponent.Play` _audio_spikes 0.0))

(fn `SetTrapPoisitonForClipping`
  (bind _spikes (`self.Spikes`))
  (`MeshComponent.SetVectorParameterValueOnMaterials` _spikes "ClipPosition" (`self.K2_GetActorLocation`))
  (`MeshComponent.SetVectorParameterValueOnMaterials` _spikes "ClipUpVector" (`self.GetActorUpVector`)))

(fn `SpikeDeploymentSpeed`
  (params (DeploymentSpeed :type "Float (double-precision)" :default 0.1))
  (`TimelineComponent.SetPlayRate` (`self.TL_DeploySpikes`) (/ 1.0 DeploymentSpeed)))

(fn `UserConstructionScript`
  (bind _triggercollisionheight (`self.TriggerCollisionHeight`))
  (bind _paincollision (`self.PainCollision`))
  (bind _platform (`self.Platform`))
  (bind _spikes (`self.Spikes`))
  (bind _triggercollision (`self.TriggerCollision`))
  (bind (_min _max) (`StaticMeshComponent.GetLocalBounds` _spikes))
  (bind _returnvalue (+ (* (/ (- _max _min) 2) (.scale (`InstancedStaticMeshComponent.GetInstanceTransform` _spikes 0 false))) (`KismetMathLibrary.MakeVector` (* (- (`self.SpikeGridSizeX`) 1) (`self.Spacing`) 0.5) (* (- (`self.SpikeGridSizeY`) 1) (`self.Spacing`) 0.5))))
  (bind _returnvalue_2 (+ _returnvalue (`self.PlatformSizeBuffer`)))
  (bind (_returnvalue_x _returnvalue_y) (`KismetMathLibrary.BreakVector` (/ _returnvalue_2 50)))
  ; Create dynamic spikes layout and adjust PainCollision to automatically fit the bounds of the spikes
  (`self.CreateSpikes`)
  (`BoxComponent.SetBoxExtent` _paincollision _returnvalue true)
  (`SceneComponent.K2_SetRelativeLocation` _paincollision (`KismetMathLibrary.MakeVector` 0.0 0.0 (.z _returnvalue)) false false)
  ; Set size and visibility of platform
  (`SceneComponent.SetRelativeScale3D` _platform (`KismetMathLibrary.MakeVector` _returnvalue_x _returnvalue_y 0.05))
  (`SceneComponent.SetHiddenInGame` _platform (`self.HidePlatform`) false)
  ; Set Size and location of TriggerCollision
  (`BoxComponent.SetBoxExtent` _triggercollision (`KismetMathLibrary.MakeVector` (.x _returnvalue_2) (.y _returnvalue_2) _triggercollisionheight) true)
  (`SceneComponent.K2_SetRelativeLocation` _triggercollision (`KismetMathLibrary.MakeVector` 0.0 0.0 _triggercollisionheight) false false)
  ; Set if spikes are intially deployed
  (`SceneComponent.K2_SetRelativeLocation` (`self.SpikesActor`) (`KismetMathLibrary.MakeVector` 0.0 0.0 (select `bool` (`self.SpikesDeployed`) :`false` -100.0)) false false)
  (`self.SetTrapPoisitonForClipping`)
  (`self.EnablePainCollision` (`self.SpikesDeployed`)))