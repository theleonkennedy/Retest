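; Spear projectile for traps that damages what it strikes and becomes a platform characters can jump on.
; Construction randomizes launch speed around ProjectileSpeed, and collision is enabled shortly after BeginPlay to avoid hits on spawn.
; Overlaps apply damage to pawns and other actors.
; The first blocking hit, gated by DoOnce, applies damage, plays an impact sound and switches the Pawn response to Block so embedded spears can be stood on.
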(event `self.ReceiveBeginPlay`
  (`KismetSystemLibrary.Delay` 0.2) ; Prevents spears from hitting objects \ndirectly then when spawing
  (`PrimitiveComponent.SetCollisionEnabled` (`self.Collision`) "QueryAndPhysics"))

(event `self.Collision.OnComponentHit`
  (params (HitComponent :type "PrimitiveComponent Object Reference") (OtherActor :type "Actor Object Reference") (OtherComp :type "PrimitiveComponent Object Reference") (NormalImpulse :type "Vector Structure") (Hit :type "HitResult Structure (by ref)"))
  ; Apply damage to hit actors to account for wanting to damage or destroy world objects
  ; // Play sounds when hitting object
  ; //Change collision response for Pawns to block to characters can jump on the embedded spears
  (`/Engine/EditorBlueprintResources/StandardMacros.DoOnce` false
    (:`Completed`
      (`GameplayStatics.ApplyDamage` OtherActor (`self.Damage`))
      (`AudioComponent.Play` (`self.Audio_HitObject`) 0.0)
      (`PrimitiveComponent.SetCollisionResponseToChannel` (`self.Collision`) "ECC_Pawn" "ECR_Block"))))

(event `self.Collision.OnComponentBeginOverlap`
  (params (OverlappedComponent :type "PrimitiveComponent Object Reference") (OtherActor :type "Actor Object Reference") (OtherComp :type "PrimitiveComponent Object Reference") (OtherBodyIndex :type Integer) (bFromSweep :type Boolean) (SweepResult :type "HitResult Structure (by ref)"))
  ; Damage pawns and other overlapping actors
  (`GameplayStatics.ApplyDamage` OtherActor (`self.Damage`)))

(fn `SetProjectileMovement`
  (bind _projectilemovement (`self.ProjectileMovement`))
  (bind _output_get (set `ProjectileMovementComponent.InitialSpeed` (* (`self.ProjectileSpeed`) (`KismetMathLibrary.RandomFloatInRange` 0.75 1.5)) _projectilemovement))
  (set `ProjectileMovementComponent.MaxSpeed` _output_get _projectilemovement))

(fn `UserConstructionScript`
  (`self.SetProjectileMovement`))