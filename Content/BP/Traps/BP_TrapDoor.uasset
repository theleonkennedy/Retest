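; Trap door that drops when a Character overlaps its collision box while armed, then resets after a delay.
; An optional TrapTrigger actor arms it through its activation event.
; A timeline rotates the platform's anchor to swing the floor down and reverses to raise it, with separate drop and reset speeds.
; The construction script sizes and hinges the platform from the collision extents and sets a grey or actor-matched material.
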(event `self.ReceiveBeginPlay`
  ; Arm trap from trigger
  (bind _traptrigger (`self.TrapTrigger`)
    (:`then`
      (add `/Game/BP/Traps/BP_TrapTrigger.OnActivateTrap` _traptrigger (delegate `OnActivateTrap_Event`)))
    (:`else`)))

(event `OnActivateTrap_Event`
  ; Arm trap from trigger
  (set `self.IsArmed` true))

(event `self.Collision.OnComponentBeginOverlap`
  (params (OverlappedComponent :type "PrimitiveComponent Object Reference") (OtherActor :type "Actor Object Reference") (OtherComp :type "PrimitiveComponent Object Reference") (OtherBodyIndex :type Integer) (bFromSweep :type Boolean) (SweepResult :type "HitResult Structure (by ref)"))
  ; Drop trap door when triggered by character
  (cast `Character` OtherActor)
  (if (and (`self.IsArmed`) (not (`self.FloorDropped`)))
    (`KismetSystemLibrary.Delay` (`self.DelayBeforeDrop`))
    (`self.TrapDoorSpeed` (`self.FloorDropSpeed`))
    (`TimelineComponent.Play` (`self.TL_DropFloor`))))

(fn `SetOverrideMaterial`
  (bind _actormatieraltomatch (`self.ActorMatieralToMatch`))
  (`PrimitiveComponent.SetMaterial` (`self.Platform`) 0 (select `bool` (`KismetSystemLibrary.IsValid` _actormatieraltomatch) :`false` (`PrimitiveComponent.GetMaterial` (`self.GetComponentByClass` _actormatieraltomatch "/Script/Engine.StaticMeshComponent") 0) :`true` "/Game/Materials/MI_Blockout_Grey.MI_Blockout_Grey")))

(fn `TrapDoorSpeed`
  (params (DoorSpeed :type "Float (double-precision)"))
  (`TimelineComponent.SetPlayRate` (`self.TL_DropFloor`) (/ 1.0 DoorSpeed)))

(fn `UserConstructionScript`
  (bind _platform (`self.Platform`))
  (bind _collision (`self.Collision`))
  (bind _collisionextents (`self.CollisionExtents`))
  (bind _platformanchor (`self.PlatformAnchor`))
  (bind _x (.x (`self.CollisionExtents`)))
  (bind (_returnvalue_x _returnvalue_y) (`KismetMathLibrary.BreakVector` (/ _collisionextents 50)))
  ; Set Size and location of collision
  (`BoxComponent.SetBoxExtent` _collision _collisionextents true)
  (`SceneComponent.K2_SetRelativeLocation` _collision (`KismetMathLibrary.MakeVector` 0.0 0.0 (.z _collisionextents)) false false)
  ; Set size and visibility of platform
  (`SceneComponent.SetRelativeScale3D` _platform (`KismetMathLibrary.MakeVector` _returnvalue_x _returnvalue_y 0.05))
  (`SceneComponent.SetHiddenInGame` _platform (`self.HidePlatform`) false)
  (`SceneComponent.K2_SetRelativeLocation` _platform (`KismetMathLibrary.MakeVector` _x) false false)
  ; Set rotation and location of platforn anchor
  (`SceneComponent.K2_SetRelativeLocation` _platformanchor (`KismetMathLibrary.MakeVector` (* _x -1.0)) false false)
  (`SceneComponent.K2_SetRelativeRotation` _platformanchor (`KismetMathLibrary.SelectRotator` (struct :`Pitch` -90.0) (struct) (`self.FloorDropped`)) false false)
  (`SceneComponent.K2_SetWorldRotation` :`self` (`self.TextRender`)) ; Prevents text from spinning
  (`self.SetOverrideMaterial`) ; Create ovverrride material, based on \nselecting a statsic mesh in the world
)