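; Spline-path elevator where each spline point is a floor, selected from a console widget built at runtime.
; Interacting while the player overlaps the collision box opens the console; choosing a floor drives a timeline at constant speed, optionally following path yaw, with audio and HUD notifications.
; The construction script sizes the platform and previews stops with instanced ghost meshes.
; SpawnCallButtons can place a call button per stop, but nothing here invokes it.
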(event `self.ReceiveBeginPlay`
  ; Move elevator
)

(event `MoveElevator`
  (bind _spline (`self.Spline`))
  (bind _spline_2 (`self.Spline`))
  (bind _platformanchor (`self.PlatformAnchor`))
  ; Move elevator
  (if (!= (`self.DestinationPoint`) (`self.CurrentPoint`))
    (`self.SetMovementSpeed`)
    (`AudioComponent.Play` (`self.Audio_Elevator`) 0.0)
    (`self.CallNotification` "Elevator on the way")
    (bind (_direction _alpha) (`Timeline|TL_MoveElevator`)
      (:`Update`
        (if (`self.PlatformRotationFollowpath`)
          (bind _returnvalue (`KismetMathLibrary.Lerp` (`SplineComponent.GetDistanceAlongSplineAtSplinePoint` _spline (`self.CurrentPoint`)) (`SplineComponent.GetDistanceAlongSplineAtSplinePoint` _spline (`KismetMathLibrary.Min` (`self.DestinationPoint`) (- (`SplineComponent.GetNumberOfSplinePoints` _spline) 1))) _alpha))
          (bind _returnvalue_2 (`SplineComponent.GetLocationAtDistanceAlongSpline` _spline_2 _returnvalue "Local"))
          (bind (_returnvalue_roll _returnvalue_pitch _returnvalue_yaw) (`KismetMathLibrary.BreakRotator` (`SplineComponent.GetRotationAtDistanceAlongSpline` _spline_2 _returnvalue "Local")))
          (`SceneComponent.K2_SetRelativeLocationAndRotation` _platformanchor _returnvalue_2 (`KismetMathLibrary.MakeRotator` 0.0 0.0 _returnvalue_yaw) false false)
          (else
            (`SceneComponent.K2_SetRelativeLocation` _platformanchor _returnvalue_2 false false))))
      (:`Finished`
        (set `self.CurrentPoint` (`self.DestinationPoint`))
        (`AudioComponent.Stop` (`self.Audio_Elevator`))))
    (else
      (`self.CallNotification` "Elevator already on this floor"))))

(event `/Game/BP/Interfaces/BPI_Interaction.Interact`
  ; Activate elevator using button
  (`/Engine/EditorBlueprintResources/StandardMacros.Gate` true :!label _label
    (:`Exit`
      (if (`TimelineComponent.IsPlaying` (`self.TL_MoveElevator`))
        (`self.CallNotification` "Elevator in motion. Please wait")
        (else
          (`self.ActivateElevatorPanel`))))))

(event `self.Collision.OnComponentBeginOverlap`
  (params (OverlappedComponent :type "PrimitiveComponent Object Reference") (OtherActor :type "Actor Object Reference") (OtherComp :type "PrimitiveComponent Object Reference") (OtherBodyIndex :type Integer) (bFromSweep :type Boolean) (SweepResult :type "HitResult Structure (by ref)"))
  ; Activate elevator using button
  (if (== (`GameplayStatics.GetPlayerCharacter` 0) OtherActor)
    (goto _label :!via `Open`)))

(event `self.Collision.OnComponentEndOverlap`
  (params (OverlappedComponent :type "PrimitiveComponent Object Reference") (OtherActor :type "Actor Object Reference") (OtherComp :type "PrimitiveComponent Object Reference") (OtherBodyIndex :type Integer))
  ; Activate elevator using button
  (if (== (`GameplayStatics.GetPlayerCharacter` 0) OtherActor)
    (goto _label :!via `Close`)))

(event `ActivateElevatorPanel`
  ; Add elevator panel
  ;; Create console widget // add button to console for each stop (measured by spline points)
  (bind _returnvalue (`|CreateWidget` "/Game/UI/WBP_ElevatorConsole.WBP_ElevatorConsole_C"))
  (set `self.WBP_ElevatorConsole` _returnvalue)
  (for _index (range (`SplineComponent.GetNumberOfSplinePoints` (`self.Spline`)))
    (bind _returnvalue_2 (`|CreateWidget` "/Game/UI/WBP_ElevatorFloorConsole.WBP_ElevatorFloorConsole_C" null _index))
    (`PanelWidget.AddChild` (`/Game/UI/WBP_ElevatorConsole.VBOX_ButtonLayout` (`self.WBP_ElevatorConsole`)) _returnvalue_2)
    (`TextBlock.SetText` (`/Game/UI/WBP_ElevatorFloorConsole.ButtonText` _returnvalue_2) (`|FormatText` "Floor {x}" _index))
    ;; Bind event for each button added to the console
    (add `/Game/UI/WBP_ElevatorFloorConsole.OnSetDestinationFloor` _returnvalue_2 (delegate `OnSetDestinationFloor_Event`)))
  ;; Add elevtor consoke to screen
  (`UserWidget.AddToViewport` (`self.WBP_ElevatorConsole`) 0))

(event `OnSetDestinationFloor_Event`
  (params (FloorIndex :type Integer))
  ; Add elevator panel
  ;; Bind event for each button added to the console
  (set `self.DestinationPoint` FloorIndex)
  (`self.MoveElevator`)
  (`Widget.RemoveFromParent` (`self.WBP_ElevatorConsole`)))

(event `SpawnCallButtons`
  (bind _spline (`self.Spline`))
  ; Auto-spawn call buttons at each stop for the elevator
  (for _index (range (`SplineComponent.GetNumberOfSplinePoints` _spline))
    (bind _returnvalue (`|SpawnActorFromClass` "/Game/BP/Equipment/BP_Advanced_ElevatorSimple_CallButton1.BP_Advanced_ElevatorSimple_CallButton1_C" (`KismetMathLibrary.Conv_VectorToTransform` (`SplineComponent.GetLocationAtSplinePoint` _spline _index "World")) "Undefined" "MultiplyWithRoot" null _index null))
    (`KismetArrayLibrary.Array_Add` (`self.CallButtons`) _returnvalue)))

(fn `CallNotification`
  (params (NotificationText :type Text))
  (message `/Game/BP/Interfaces/BPI_Interaction.UpdateHUD_Notification` (`GameplayStatics.GetPlayerController` 0) NotificationText))

(fn `GetInteractionInfo`
  (returns (InteractionInfo :type Text))
  (return "move elevator"))

(fn `SetMovementSpeed`
  (bind _spline (`self.Spline`))
  ; Set movement speed of the elevator
  (`TimelineComponent.SetPlayRate` (`self.TL_MoveElevator`) (/ 1.0 (/ (`KismetMathLibrary.Abs` (- (`SplineComponent.GetDistanceAlongSplineAtSplinePoint` _spline (`self.CurrentPoint`)) (`SplineComponent.GetDistanceAlongSplineAtSplinePoint` _spline (`KismetMathLibrary.Min` (`self.DestinationPoint`) (- (`SplineComponent.GetNumberOfSplinePoints` _spline) 1))))) (`self.Speed`)))))

(fn `UpdateGhostPlatforms`
  (bind _platformghost (`self.PlatformGhost`))
  (bind (_returnvalue_location _returnvalue_rotation _returnvalue_scale) (`KismetMathLibrary.BreakTransform` (`SceneComponent.GetRelativeTransform` (`self.Platform`))))
  (`StaticMeshComponent.SetStaticMesh` _platformghost (`StaticMeshComponent.StaticMesh` (`self.Platform`)))
  (`PrimitiveComponent.SetMaterial` _platformghost 0 "/Game/Materials/MI_PlatformGhost.MI_PlatformGhost")
  (for _index (range (`SplineComponent.GetNumberOfSplinePoints` (`self.Spline`)))
    (`InstancedStaticMeshComponent.AddInstance` _platformghost (`KismetMathLibrary.MakeTransform` (`SplineComponent.GetLocationAtSplinePoint` (`self.Spline`) _index "World") _returnvalue_rotation _returnvalue_scale) true)))

(fn `UserConstructionScript`
  (bind _collision (`self.Collision`))
  (bind _collisionextents (`self.CollisionExtents`))
  (bind (_returnvalue_x _returnvalue_y) (`KismetMathLibrary.BreakVector` (/ _collisionextents 50)))
  ; Set Size and location of collision
  (`BoxComponent.SetBoxExtent` _collision _collisionextents true)
  (`SceneComponent.K2_SetRelativeLocation` _collision (`KismetMathLibrary.MakeVector` 0.0 0.0 (.z _collisionextents)) false false)
  ; Set size and visibility of platform
  (`SceneComponent.SetRelativeScale3D` (`self.Platform`) (`KismetMathLibrary.MakeVector` _returnvalue_x _returnvalue_y 0.05))
  ; Move and control panel to edge of platform when resizing
  (`SceneComponent.K2_SetRelativeLocation` (`self.ControlPanelAnchor`) (`KismetMathLibrary.MakeVector` (- (.x _collisionextents) 6.0)) false false)
  ; Set path color for spline
  (`SplineComponent.SetUnselectedSplineSegmentColor` (`self.Spline`) (`self.PathColor`))
  (`self.UpdateGhostPlatforms`))