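; Interactable light switch that toggles a selected set of lights on and off.
; Interact loops over the Lights array and flips the visibility of each valid light's LightComponent individually, so lights in mixed states swap rather than sync.
; GetInteractionInfo supplies the "toggle lights" text describing the interaction.
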(event `/Game/BP/Interfaces/BPI_Interaction.Interact`
  (bind _lights (`self.Lights`))
  ; Toggles selected lights in array on and off
  (if (`KismetArrayLibrary.Array_IsValidIndex` _lights)
    (for _array_element _lights
      (`/Engine/EditorBlueprintResources/StandardMacros.IsValid` _array_element
        (:`Is Valid`
          (bind _lightcomponent (`Light.LightComponent` _array_element))
          (`SceneComponent.SetVisibility` _lightcomponent (not (`SceneComponent.IsVisible` _lightcomponent)) false))))))

(fn `GetInteractionInfo`
  (returns (InteractionInfo :type Text))
  (return "toggle lights"))

(fn `UserConstructionScript`)