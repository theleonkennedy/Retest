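; Single swinging door Blueprint, toggled by interaction or optionally triggered by the player overlapping a resizable collision box.
; DoorHandler picks the swing side from a player-to-forward dot product, restarts a timeline scaled by OpenCloseTime, and updates the interaction text.
; Both overlap begin and end set the door to open.
; The rotation-lerp update sits in an unexecuted block, with a hardcoded false select that zeroes the open angle.
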(event `self.ReceiveBeginPlay`
  ; Set how long the door takes to open and close
  (`TimelineComponent.SetPlayRate` (`self.TL_OpenCloseDoor`) (/ 1.0 (`self.OpenCloseTime`)))
  ; Enable / Disable collision based on if Auto-Open is enable
  (`PrimitiveComponent.SetCollisionEnabled` (`self.Collision`) (select `bool` (`self.EnableAutoOpen`) :`false` "NoCollision" :`true` "QueryOnly" :!type "ECollisionEnabled Enum")))

(event `self.Collision.OnComponentBeginOverlap`
  (params (OverlappedComponent :type "PrimitiveComponent Object Reference") (OtherActor :type "Actor Object Reference") (OtherComp :type "PrimitiveComponent Object Reference") (OtherBodyIndex :type Integer) (bFromSweep :type Boolean) (SweepResult :type "HitResult Structure (by ref)"))
  ; Automatically open the door, if enabled
  (if (and (== OtherActor (`GameplayStatics.GetPlayerCharacter` 0)) (not (`self.OpenTheDoor`)))
    (set `self.OpenTheDoor` true)
    (`self.DoorHandler` :!label _label)))

(event `self.Collision.OnComponentEndOverlap`
  (params (OverlappedComponent :type "PrimitiveComponent Object Reference") (OtherActor :type "Actor Object Reference") (OtherComp :type "PrimitiveComponent Object Reference") (OtherBodyIndex :type Integer))
  ; Automatically open the door, if enabled
  (if (== (`GameplayStatics.GetPlayerCharacter` 0) OtherActor)
    (set `self.OpenTheDoor` true)
    (goto _label)))

(event `/Game/BP/Interfaces/BPI_Interaction.Interact`
  ; Open/Close the door through interaction
  (set `self.OpenTheDoor` (not (`self.OpenTheDoor`)))
  (`self.DoorHandler`))

(event `DoorHandler`
  (bind _tl_openclosedoor (`self.TL_OpenCloseDoor`))
  ; Handle opening / closing
  (`TimelineComponent.Stop` _tl_openclosedoor)
  (`self.CaculateDoorOpenDirection`)
  (`TimelineComponent.PlayFromStart` _tl_openclosedoor)
  ; Adjust interaction text based on if door is open or closed
  (set `self.Interaction Info` (`KismetMathLibrary.SelectText` "close the door" "open the door" (`self.OpenTheDoor`))))

(fn `CaculateDoorOpenDirection`
  (set `self.DoorOpenDirection` (>= (`KismetMathLibrary.Dot_VectorVector` (`KismetMathLibrary.Normal` (- (`self.K2_GetActorLocation`) (`self.K2_GetActorLocation` (`GameplayStatics.GetPlayerCharacter` 0)))) (`self.GetActorForwardVector`)) 0.0)))

(fn `GetInteractionInfo`
  (returns (InteractionInfo :type Text))
  (return (`self.Interaction Info`)))

(fn `UserConstructionScript`
  (bind _collision (`self.Collision`))
  (bind _collisionextents (`self.CollisionExtents`))
  (`BoxComponent.SetBoxExtent` _collision _collisionextents true)
  (`SceneComponent.K2_SetRelativeLocation` _collision (`KismetMathLibrary.MakeVector` 0.0 0.0 (.z _collisionextents)) false false))