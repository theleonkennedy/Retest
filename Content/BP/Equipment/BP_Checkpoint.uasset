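; BP_Checkpoint is a placeable checkpoint that sets the player's respawn point when they overlap its box.
; It sends the player controller a transform at the checkpoint center, raised by capsule half height and facing the Arrow.
; It then updates every checkpoint of its class, so only the current one disables its trigger, plays particles and audio, and turns green.
; The construction script drives trigger size, platform scale and visibility, and respawn direction from variables.
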(event `self.Collision.OnComponentBeginOverlap`
  (params (OverlappedComponent :type "PrimitiveComponent Object Reference") (OtherActor :type "Actor Object Reference") (OtherComp :type "PrimitiveComponent Object Reference") (OtherBodyIndex :type Integer) (bFromSweep :type Boolean) (SweepResult :type "HitResult Structure (by ref)"))
  (bind _returnvalue (`GameplayStatics.GetPlayerCharacter` 0))
  (bind (_returnvalue_x _returnvalue_y _returnvalue_z) (`KismetMathLibrary.BreakVector` (`self.K2_GetActorLocation`)))
  ; Check if player overlaps collision
  (if (== _returnvalue OtherActor)
    ; Set respawn point to center of checkpoint in the direction of the Arrow component
    (message `/Game/BP/Interfaces/BPI_PlayerInfo.SetRespawnTransform` (`GameplayStatics.GetPlayerController` 0) (`KismetMathLibrary.MakeTransform` (`KismetMathLibrary.MakeVector` _returnvalue_x _returnvalue_y (+ _returnvalue_z (`CapsuleComponent.CapsuleHalfHeight` (`Character.CapsuleComponent` _returnvalue)))) (`SceneComponent.K2_GetComponentRotation` (`self.Arrow`))))
    ; Check all checkpoints in level and deactivate if not the current checkpoint
    (bind _outactors (`GameplayStatics.GetAllActorsOfClass` (`GameplayStatics.GetObjectClass` self)))
    (for _array_element _outactors
      (`self.ActiveCheckpoint` _array_element (== _array_element self)))))

(fn `ActiveCheckpoint`
  (params (SelfCheck :type Boolean))
  (bind _selfcheck (`local.SelfCheck`))
  (`PrimitiveComponent.SetCollisionEnabled` (`self.Collision`) (select `bool` SelfCheck :`false` "QueryOnly" :`true` "NoCollision" :!type "ECollisionEnabled Enum"))
  (`ActorComponent.SetActive` (`self.ParticleSystem`) _selfcheck false)
  (`ActorComponent.SetActive` (`self.Audio`) _selfcheck false)
  (`MeshComponent.SetVectorParameterValueOnMaterials` (`self.Platform`) "FloorColor" (`KismetMathLibrary.Conv_LinearColorToVector` (select `bool` _selfcheck :`false` (struct :`R` 1.0 :`G` 1.0 :`B` 1.0 :`A` 1.0) :`true` (struct :`G` 1.0 :`A` 1.0) :!type "LinearColor Structure"))))

(fn `UserConstructionScript`
  (bind _collision (`self.Collision`))
  (bind _collisionextents (`self.CollisionExtents`))
  (bind _platform (`self.Platform`))
  (bind _hideplatform (`self.HidePlatform`))
  (bind (_returnvalue_x _returnvalue_y) (`KismetMathLibrary.BreakVector` (/ _collisionextents 50)))
  ; Set Size and location of collision
  (`BoxComponent.SetBoxExtent` _collision _collisionextents true)
  (`SceneComponent.K2_SetRelativeLocation` _collision (`KismetMathLibrary.MakeVector` 0.0 0.0 (.z _collisionextents)) false false)
  ; Set size and visibility of platform
  (`SceneComponent.SetRelativeScale3D` _platform (`KismetMathLibrary.MakeVector` _returnvalue_x _returnvalue_y 0.05))
  (`SceneComponent.SetHiddenInGame` _platform _hideplatform false)
  (`PrimitiveComponent.SetCollisionEnabled` _platform (select `bool` _hideplatform :`false` "QueryAndPhysics" :`true` "NoCollision" :!type "ECollisionEnabled Enum"))
  ; Set arrow direction for respawning
  (`SceneComponent.K2_SetRelativeRotation` (`self.Arrow`) (`KismetMathLibrary.MakeRotator` 0.0 0.0 (`self.RespawnDirection`)) false false))