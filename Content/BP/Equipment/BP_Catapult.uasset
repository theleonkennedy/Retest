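; BP_Catapult is a launch pad that throws the player character along the pad's up vector on overlap.
; Its box collision detects only player 0, then launches with a configurable strength that overrides vertical velocity, alongside an explosion particle and sound.
; The construction script sizes and raises the collision box from one extents variable, scales the thin platform mesh to match, and can hide it in game.
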(event `self.Collision.OnComponentBeginOverlap`
  (params (OverlappedComponent :type "PrimitiveComponent Object Reference") (OtherActor :type "Actor Object Reference") (OtherComp :type "PrimitiveComponent Object Reference") (OtherBodyIndex :type Integer) (bFromSweep :type Boolean) (SweepResult :type "HitResult Structure (by ref)"))
  (bind _returnvalue (`GameplayStatics.GetPlayerCharacter` 0))
  ; Launch player when they step on the pad
  (if (== _returnvalue OtherActor)
    (`GameplayStatics.SpawnEmitterAtLocation` "/Game/StarterContent/Particles/P_Explosion.P_Explosion" (`self.K2_GetActorLocation`) (struct) (3.0 3.0 3.0))
    (`Character.LaunchCharacter` _returnvalue (* (`self.GetActorUpVector`) (`self.LaunchStrenght`)) false true)
    (`GameplayStatics.PlaySoundAtLocation` "/Game/StarterContent/Audio/Explosion_Cue.Explosion_Cue" (`self.K2_GetActorLocation`) (struct) 1.0 1.0 0.0 null null null null)))

(fn `UserConstructionScript`
  (bind _collision (`self.Collision`))
  (bind _collisionextents (`self.CollisionExtents`))
  (bind _platform (`self.Platform`))
  (bind (_returnvalue_x _returnvalue_y) (`KismetMathLibrary.BreakVector` (/ _collisionextents 50)))
  ; Set Size and location of collision
  (`BoxComponent.SetBoxExtent` _collision _collisionextents true)
  (`SceneComponent.K2_SetRelativeLocation` _collision (`KismetMathLibrary.MakeVector` 0.0 0.0 (.z _collisionextents)) false false)
  ; Set size and visibility of platform
  (`SceneComponent.SetRelativeScale3D` _platform (`KismetMathLibrary.MakeVector` _returnvalue_x _returnvalue_y 0.05))
  (`SceneComponent.SetHiddenInGame` _platform (`self.HidePlatform`) false))