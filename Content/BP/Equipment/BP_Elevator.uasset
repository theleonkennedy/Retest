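; Two-floor elevator that moves a platform between its origin and a configurable MoveLocation.
; A timeline lerps the platform anchor, with play rate derived from distance and Speed, and tracks the current floor when finished.
; Two optional call buttons send it to their floor, while Interact toggles floors only while the player overlaps the collision box.
; The construction script sizes platform and collision, positions the control panel, and previews the destination with a ghost platform.
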(event `self.ReceiveBeginPlay`
  (`|ExecutionSequence`
    (:`then_0`
      ; Set movement speed of the elevator
      (`TimelineComponent.SetPlayRate` (`self.TL_MoveElevator`) (/ 1.0 (/ (`KismetMathLibrary.Vector_Distance` (`self.MoveLocation`) (`SceneComponent.RelativeLocation` (`self.PlatformAnchor`))) (`self.Speed`)))))
    (:`then_1`
      ; Bind 1st Floor call button
      (bind _callbutton_1stfloor (`self.CallButton_1stFloor`)
        (:`then`
          (add `/Game/BP/Equipment/BP_ElevatorSimple_CallButton.CallElevatorToFloor` _callbutton_1stfloor (delegate `CallElevatorToFloor_Event`)))
        (:`else`)))
    (:`then_2`
      ; Bind 2nd Floor call button
      (bind _callbutton_2ndfloor_0 (`self.CallButton_2ndFloor_0`)
        (:`then`
          (add `/Game/BP/Equipment/BP_ElevatorSimple_CallButton.CallElevatorToFloor` _callbutton_2ndfloor_0 (delegate `CallElevatorToFloor_Event_0`)))
        (:`else`)))))

(event `CallElevatorToFloor_Event`
  ; Bind 1st Floor call button
  (`self.MoveTo1stFloor`))

(event `CallElevatorToFloor_Event_0`
  ; Bind 2nd Floor call button
  (`self.MoveTo2ndFloor`))

(event `MoveTo2ndFloor`
  ; Move elevator
  (bind (_direction _alpha) (`Timeline|TL_MoveElevator` :!label _label)
    (:`Update`
      (`SceneComponent.K2_SetRelativeLocation` (`self.PlatformAnchor`) (`KismetMathLibrary.VLerp` (0.0 0.0 0.0) (`self.MoveLocation`) _alpha) false false))
    (:`Finished`
      (set `self.On1stFloor` (select `ETimelineDirection` _direction :`Backward` true)))))

(event `MoveTo1stFloor`
  ; Move elevator
  (goto _label :!via `Reverse`))

(event `/Game/BP/Interfaces/BPI_Interaction.Interact`
  ; Activate elevator using button
  (`/Engine/EditorBlueprintResources/StandardMacros.Gate` true :!label _label_2
    (:`Exit`
      (if (`self.On1stFloor`)
        (`self.MoveTo2ndFloor`)
        (else
          (`self.MoveTo1stFloor`))))))

(event `self.Collision.OnComponentBeginOverlap`
  (params (OverlappedComponent :type "PrimitiveComponent Object Reference") (OtherActor :type "Actor Object Reference") (OtherComp :type "PrimitiveComponent Object Reference") (OtherBodyIndex :type Integer) (bFromSweep :type Boolean) (SweepResult :type "HitResult Structure (by ref)"))
  ; Activate elevator using button
  (if (== (`GameplayStatics.GetPlayerCharacter` 0) OtherActor)
    (goto _label_2 :!via `Open`)))

(event `self.Collision.OnComponentEndOverlap`
  (params (OverlappedComponent :type "PrimitiveComponent Object Reference") (OtherActor :type "Actor Object Reference") (OtherComp :type "PrimitiveComponent Object Reference") (OtherBodyIndex :type Integer))
  ; Activate elevator using button
  (if (== (`GameplayStatics.GetPlayerCharacter` 0) OtherActor)
    (goto _label_2 :!via `Close`)))

(fn `GetInteractionInfo`
  (returns (InteractionInfo :type Text))
  (return "move elevator"))

(fn `UserConstructionScript`
  (bind _collision (`self.Collision`))
  (bind _collisionextents (`self.CollisionExtents`))
  (bind (_returnvalue_x _returnvalue_y) (`KismetMathLibrary.BreakVector` (/ _collisionextents 50)))
  ; Set Size and location of collision
  (`BoxComponent.SetBoxExtent` _collision _collisionextents true)
  (`SceneComponent.K2_SetRelativeLocation` _collision (`KismetMathLibrary.MakeVector` 0.0 0.0 (.z _collisionextents)) false false)
  ; Set size and visibility of platform
  (`SceneComponent.SetRelativeScale3D` (`self.Platform`) (`KismetMathLibrary.MakeVector` _returnvalue_x _returnvalue_y 0.05))
  (`SceneComponent.SetRelativeScale3D` (`self.PlatformGhost`) (`KismetMathLibrary.MakeVector` _returnvalue_x _returnvalue_y 0.05))
  ; Move and control panel to edge of platform when resizing
  (`SceneComponent.K2_SetRelativeLocation` (`self.ControlPanelAnchor`) (`KismetMathLibrary.MakeVector` (- (.x _collisionextents) 6.0)) false false)
  ; Show placement of elevator move desitination
  (`SceneComponent.K2_SetRelativeLocation` (`self.PlatformGhost`) (`self.MoveLocation`) false false))