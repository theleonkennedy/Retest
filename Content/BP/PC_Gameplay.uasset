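; PC_Gameplay is the gameplay player controller that owns the HUD and relays text to it.
; On BeginPlay it creates WBP_HUD, stores the reference and adds it to the viewport.
; Two events forward interaction and notification text to that widget, while GetInteractionInfo is a stub that returns an empty string.
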(event `self.ReceiveBeginPlay`
  ; Create HUD and add it to the screen
  (bind _returnvalue (`|CreateWidget` "/Game/UI/WBP_HUD.WBP_HUD_C"))
  (bind _output_get (set `self.WBP_HUD` _returnvalue))
  (`UserWidget.AddToViewport` _output_get 0))

(event `/Game/BP/Interfaces/BPI_INTERACTION.UpdateHUD_Interaction`
  (params (InteractionText :type Text))
  ; Interaction
  ;; Update HUD Interaction Text
  (`/Game/UI/WBP_HUD.UpdateInteractionText` (`self.WBP_HUD`) InteractionText))

(event `/Game/BP/Interfaces/BPI_INTERACTION.UpdateHUD_Notification`
  (params (NotificationText :type Text))
  ; Interaction
  ;; Update HUD Notication Text
  (`/Game/UI/WBP_HUD.UpdateNoticatiionText` (`self.WBP_HUD`) NotificationText))

(fn `GetInteractionInfo`
  (returns (InteractionInfo :type Text))
  (return ""))

(fn `UserConstructionScript`)